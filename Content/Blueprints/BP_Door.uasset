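; BP_Door is a door that a BP_ThirdPersonCharacter opens by interacting and that closes when the character leaves its Box trigger.
; BeginPlay caches the door's world yaw, and the DoorOpening timeline lerps from it to 90 degrees less.
; OpenDoor plays the timeline and CloseDoor reverses it.
; A comment marks OpenDoor as multicast so all clients see the effect.
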(event `self.ReceiveBeginPlay`
  (bind (_returnvalue_roll _returnvalue_pitch _returnvalue_yaw) (`KismetMathLibrary.BreakRotator` (`SceneComponent.K2_GetComponentRotation` (`self.Door`))))
  (set `self.Z_Rotation` _returnvalue_yaw))

(event `/Game/Blueprints/InteractInterface.Interacted`
  (params (Interactor :type "Actor Object Reference"))
  (cast `/Game/ThirdPerson/Blueprints/BP_ThirdPersonCharacter` Interactor)
  (`self.OpenDoor`))

(event `self.Box.OnComponentEndOverlap`
  (params (OverlappedComponent :type "PrimitiveComponent Object Reference") (OtherActor :type "Actor Object Reference") (OtherComp :type "PrimitiveComponent Object Reference") (OtherBodyIndex :type Integer))
  (cast `/Game/ThirdPerson/Blueprints/BP_ThirdPersonCharacter` OtherActor)
  (`self.CloseDoor`))

(event `OpenDoor`
  (bind _z_rotation (`self.Z_Rotation`))
  ;[0 0 0] Multicast because we want all clients to see this effect
  (bind (_direction _doorposition) (`Timeline|DoorOpening` :!label _label)
    (:`Update`
      (`SceneComponent.K2_SetWorldRotation` (`self.Door`) (`KismetMathLibrary.MakeRotator` 0.0 0.0 (`KismetMathLibrary.Lerp` _z_rotation (+ _z_rotation -90.0) _doorposition)) false false))))

(event `CloseDoor`
  ;[0 0 0] Multicast because we want all clients to see this effect
  (goto _label :!via `Reverse`))

(fn `UserConstructionScript`)