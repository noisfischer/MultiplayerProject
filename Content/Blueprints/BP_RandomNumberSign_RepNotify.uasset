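; Replicated sign actor that shows a server-generated random number, demonstrating RepNotify variables.
; On the server, a looping timer rolls a new random float, and its OnRep function writes the value to a text render component.
; The construction script sizes a sphere to the actor's net cull distance to visualise relevancy range.
; An empty multicast effects event is stubbed in, with a note that only relevant clients receive it.
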(event `self.ReceiveBeginPlay`
  (`/Engine/EditorBlueprintResources/ActorMacros.Switch Has Authority` ; Authority = Server, Remote = Client
    (:`Authority`
      (`KismetSystemLibrary.K2_SetTimerDelegate` (delegate `Update`) 1.0 true))))

(event `Update`
  (set `self.RandomFloat` (`KismetMathLibrary.RandomFloatInRange` 0.0 10.0)))

(event `MC_Effects`)

(fn `OnRep_RandomFloat`
  (`TextRenderComponent.K2_SetText` (`self.TextRender`) (`KismetTextLibrary.Conv_DoubleToText` (`self.RandomFloat`) "HalfToEven")))

(fn `UserConstructionScript`
  (`SphereComponent.SetSphereRadius` (`self.NetCullDistance`) (`KismetMathLibrary.Sqrt` (`self.NetCullDistanceSquared`)) true))